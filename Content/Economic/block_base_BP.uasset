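; Base block actor for the economic simulation, a clickable cube that represents one terrain block from the Python simulation.
; Construction picks a material from CubeType, a C++ mirror of the Python block enum, and caches it as the default.
; Simulation data updates swap in a bush material while the block is blooming.
; Cursor hover highlights the cube, and clicks are forwarded to Econ_PC.BlockClicked.
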(event OnClicked(Cube)
  (params (TouchedComponent :type Primitive%20Component%20Object%20Reference) (ButtonPressed :type Key%20Structure :default "AnyKey"))
  (bind _asecon_pc (Utilities|Casting|CastToEcon_PC (Game|GetPlayerController 0)))
  (Default|BlockClicked _asecon_pc self))

(event EventPythonSimulationNewEvent
  (params (game_event :type Py%20Sim%20Game%20Event%20Structure)))

(event MouseInput|EventActorEndCursorOver
  ;[1 1 1] Simple highlighting
  (Variables|Default|SetisHighlighted false)
  (Rendering|Material|SetMaterial (Variables|Default|GetCube) 0 (Variables|Default|GetMyDefaultMaterial)))

(event MouseInput|EventActorBeginCursorOver
  ;[1 1 1] Simple highlighting
  (Variables|Default|SetisHighlighted true)
  (Rendering|Material|SetMaterial (Variables|Default|GetCube) 0 "/Game/StarterContent/Materials/M_Basic_Floor.M_Basic_Floor"))

(event EventPythonSimulationDataUpdate
  (params (behaviour_role :type Integer))
  (bind _cube (Variables|Default|GetCube))
  (if (.is_blooming (Variables|Default|Getbeh_blooming))
    (Rendering|Material|SetMaterial _cube 0 "/Game/StarterContent/Props/Materials/M_Bush.M_Bush")
    (else
      (Rendering|Material|SetMaterial _cube 0 (Variables|Default|GetMyDefaultMaterial)))))

(fn ConstructionScript
  (CallFunction|SetMaterialBasedonCubeType)
  (Variables|Default|SetMyDefaultMaterial (Rendering|Material|GetMaterial (Variables|Default|GetCube) 0)))

(fn SetMaterialBasedonCubeType
  (bind _cube (Variables|Default|GetCube))
  (switch int (Variables|Default|Getcube_type) ; Refer to python enumeration to read this
    (:0
      (Rendering|Material|SetMaterial _cube 0 "/Game/StarterContent/Props/Materials/M_Door.M_Door") ; Error (helps to control deffered spawn\nas  well since this is a default value
    )
    (:1
      (Rendering|Material|SetMaterial _cube 0 "/Game/StarterContent/Materials/M_CobbleStone_Pebble.M_CobbleStone_Pebble") ; blRock
    )
    (:2
      (Rendering|Material|SetMaterial _cube 0 "/Game/StarterContent/Materials/M_Ground_Grass.M_Ground_Grass") ; blSoil
    )
    (:3
      (Rendering|Material|SetMaterial _cube 0 "/Game/StarterContent/Materials/M_Metal_Rust.M_Metal_Rust") ; blSand
    )
    (:4
      (Rendering|Material|SetMaterial _cube 0 "/Game/StarterContent/Materials/M_Water_Lake.M_Water_Lake") ; blWater
    )))